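; TriggerBox is a Blueprint that teleports the first-person character to a fixed location when Interact fires.
; Overlapping Box caches the character reference used by the teleport.
; Box1 enables player input on the actor and removes all widgets on entry, then disables input on exit.
; Interact also activates four audio components after the move.
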(event OnComponentBeginOverlap(Box)
  (params (OverlappedComponent :type Primitive%20Component%20Object%20Reference) (OtherActor :type Actor%20Object%20Reference) (OtherComp :type Primitive%20Component%20Object%20Reference) (OtherBodyIndex :type Integer) (bFromSweep :type Boolean) (SweepResult :type Hit%20Result%20Structure%20%28by%20ref%29))
  (bind _asfirst_person_character (Utilities|Casting|CastToFirstPersonCharacter OtherActor)))

(event OnComponentEndOverlap(Box1)
  (params (OverlappedComponent :type Primitive%20Component%20Object%20Reference) (OtherActor :type Actor%20Object%20Reference) (OtherComp :type Primitive%20Component%20Object%20Reference) (OtherBodyIndex :type Integer))
  (Utilities|Casting|CastToFirstPersonCharacter OtherActor)
  (Input|DisableInput (Game|GetPlayerController 0)))

(event OnComponentBeginOverlap(Box1)
  (params (OverlappedComponent :type Primitive%20Component%20Object%20Reference) (OtherActor :type Actor%20Object%20Reference) (OtherComp :type Primitive%20Component%20Object%20Reference) (OtherBodyIndex :type Integer) (bFromSweep :type Boolean) (SweepResult :type Hit%20Result%20Structure%20%28by%20ref%29))
  (Utilities|Casting|CastToFirstPersonCharacter OtherActor)
  (Input|EnableInput (Game|GetPlayerController 0))
  (Viewport|RemoveAllWidgets))

(event EventInteract
  (Transformation|SetWorldLocation (Variables|/Script/Engine.Actor|GetRootComponent (stale OnComponentBeginOverlap(Box) _asfirst_person_character)) "-460.000000,770.000000,-170.000000" false true)
  (Components|Activation|SetActive (Variables|Default|GetAudio) true false))

(fn ConstructionScript)